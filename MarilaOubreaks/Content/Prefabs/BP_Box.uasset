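; BP_Box is a damageable box that drops loot when destroyed.
; AnyDamage lowers a clamped Health value; at zero it calls DropLoot and destroys the actor.
; DropLoot line-traces down to find the ground, then spawns one of two loot classes at a random reachable nav point near the hit, with random yaw.
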(event `self.ReceiveAnyDamage`
  (params (Damage :type "Float (single-precision)") (DamageType :type "DamageType Object Reference") (InstigatedBy :type "Controller Object Reference") (DamageCauser :type "Actor Object Reference"))
  ;[1 1 1] Player damage on box
  (bind _output_get (set `self.Health` (`KismetMathLibrary.FClamp` (- (`self.Health`) Damage) 0.0 100.0)))
  (if (== _output_get 0.0)
    (for _ (range (+ (`KismetMathLibrary.RandomInteger` 1) 1))
      (`self.Drop Loot`))
    (`self.K2_DestroyActor`)))

(event `Drop Loot`
  (bind _returnvalue (`self.K2_GetActorLocation`))
  (bind _outhit (`KismetSystemLibrary.LineTraceSingle` _returnvalue (- _returnvalue (0.0 0.0 200.0)) "TraceTypeQuery1" false (`|MakeArray` (`GameplayStatics.GetPlayerCharacter` 0) :!type "Actor Object Reference")))
  (`|SpawnActorFromClass` (select `int` (`KismetMathLibrary.RandomInteger` 2) :`0` "/Game/Prefabs/BP_Loot_1.BP_Loot_1_C" :`1` "/Game/Prefabs/BP_Loot_2.BP_Loot_2_C" :!type "Actor Class Reference") (`KismetMathLibrary.MakeTransform` (`NavigationSystemV1.K2_GetRandomReachablePointInRadius` (`.Location` (`GameplayStatics.BreakHitResult` _outhit)) 100.0 null null) (`KismetMathLibrary.MakeRotator` 0.0 0.0 (`KismetMathLibrary.RandomFloatInRange` 0.0 360.0))) "Undefined" "OverrideRootScale" null null))

(fn `UserConstructionScript`)