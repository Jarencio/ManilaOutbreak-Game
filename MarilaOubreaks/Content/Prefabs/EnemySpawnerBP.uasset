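; Enemy spawner actor that repeatedly spawns waves of a configurable enemy class at its own transform.
; On BeginPlay it calls SpawnEnemy, which spawns NumberOfEnemy actors in a single loop, all at the same transform.
; The event then waits SpawnDelay and calls itself again with the spawner's current transform, so waves repeat with no stop condition or cap on live enemies.
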(event `self.ReceiveBeginPlay`
  (`self.Spawn Enemy` (`self.Enemy`) (`self.GetTransform`) (`self.Number of Enemy`)))

(event `Spawn Enemy`
  (params (Enemy :type "Actor Class Reference") (SpawnTransform :type "Transform Structure") (`Number of Enemy` :type Integer))
  (for _ (range `Number of Enemy`)
    (`|SpawnActorFromClass` Enemy SpawnTransform "Undefined" "OverrideRootScale" null null))
  (`KismetSystemLibrary.Delay` (`self.Spawn Delay`))
  (`self.Spawn Enemy` (`self.Enemy`) (`self.GetTransform`) (`self.Number of Enemy`)))

(fn `UserConstructionScript`)