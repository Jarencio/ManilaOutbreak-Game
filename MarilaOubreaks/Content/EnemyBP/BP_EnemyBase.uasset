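; Base enemy actor that chases seen pawns, attacks in melee and is destroyed when damage drops its clamped health to zero.
; Pawn sensing drives AI MoveTo toward the target, and a retriggerable delay halts the chase once sightings stop.
; Reaching the target triggers a sphere overlap that damages third-person characters.
; A radius overlap sets a looping zero-time timer event intended to smoothly yaw toward the character.
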(event `self.ReceiveAnyDamage`
  (params (Damage :type "Float (single-precision)") (DamageType :type "DamageType Object Reference") (InstigatedBy :type "Controller Object Reference") (DamageCauser :type "Actor Object Reference"))
  ;[1 1 1] Player damage on enemy
  (bind _output_get (set `self.Health` (`KismetMathLibrary.FClamp` (- (`self.Health`) Damage) 0.0 100.0)))
  (if (== _output_get 0.0)
    (`self.K2_DestroyActor`)))

(event `self.PawnSensing.OnSeePawn`
  (params (Pawn :type "Pawn Object Reference"))
  ;[1 1 1] Chase
  (`|ExecutionSequence`
    (:`then_0`
      (`|AIMoveTo` self (0.0 0.0 0.0) Pawn
        (:`OnSuccess`
          (`self.Attack`))))
    (:`then_1`
      (`KismetSystemLibrary.RetriggerableDelay` 1.0)
      (`|AIMoveTo` null (`self.K2_GetActorLocation`) null))))

(event `Attack`
  ;[1 1 1] Enemy attack
  (bind _outactors (`KismetSystemLibrary.SphereOverlapActors` (`SceneComponent.K2_GetComponentLocation` (`self.AttackRadius`)) 50.0 (`|MakeArray` "ObjectTypeQuery3" :!type "EObjectTypeQuery Enum") "/Game/ThirdPersonBP/Blueprints/ThirdPersonCharacter.ThirdPersonCharacter_C"))
  (for _array_element _outactors
    (`GameplayStatics.ApplyDamage` _array_element (`self.Damage`) null self)))

(event `self.LookAtPlayerRadius.OnComponentBeginOverlap`
  (params (OverlappedComponent :type "PrimitiveComponent Object Reference") (OtherActor :type "Actor Object Reference") (OtherComp :type "PrimitiveComponent Object Reference") (OtherBodyIndex :type Integer) (bFromSweep :type Boolean) (SweepResult :type "HitResult Structure (by ref)"))
  ;[1 1 1] Look at Player
  (bind _ascharacter (cast `Character` OtherActor))
  (set `self.Char Reference` _ascharacter)
  (bind _returnvalue (`KismetSystemLibrary.K2_SetTimerDelegate` (delegate `Rotate`) 0.0 true))
  (set `self.NewVar_1` _returnvalue))

(event `Rotate`
  (bind (_returnvalue_roll _returnvalue_pitch _returnvalue_yaw) (`KismetMathLibrary.BreakRotator` (`KismetMathLibrary.RInterpTo` (`self.K2_GetActorRotation`) (`KismetMathLibrary.FindLookAtRotation` (`self.K2_GetActorLocation`) (`self.K2_GetActorLocation` (`self.Char Reference`))) (`GameplayStatics.GetWorldDeltaSeconds`) 10.0)))
  ;[1 1 1] Look at Player
  (`self.K2_SetActorRotation` (`KismetMathLibrary.MakeRotator` 0.0 0.0 _returnvalue_yaw)))

(fn `UserConstructionScript`)