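; Enemy base Blueprint that chases seen pawns and is meant to turn toward nearby characters.
; PawnSensing drives AI MoveTo, while a retriggerable one-second delay halts the chase at the enemy's current location once sightings stop.
; Sphere overlap stores the character and requests a looping timer for yaw-only interpolated look-at, but its zero interval means Unreal never schedules it.
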(event `self.PawnSensing.OnSeePawn`
  (params (Pawn :type "Pawn Object Reference"))
  ;[1 1 1] Chase
  (`|ExecutionSequence`
    (:`then_0`
      (`|AIMoveTo` self (0.0 0.0 0.0) Pawn))
    (:`then_1`
      (`KismetSystemLibrary.RetriggerableDelay` 1.0)
      (`|AIMoveTo` null (`self.K2_GetActorLocation`) null))))

(event `self.Sphere.OnComponentBeginOverlap`
  (params (OverlappedComponent :type "PrimitiveComponent Object Reference") (OtherActor :type "Actor Object Reference") (OtherComp :type "PrimitiveComponent Object Reference") (OtherBodyIndex :type Integer) (bFromSweep :type Boolean) (SweepResult :type "HitResult Structure (by ref)"))
  ;[1 1 1] Look at Player
  (bind _ascharacter (cast `Character` OtherActor))
  (set `self.Char Reference` _ascharacter)
  (bind _returnvalue (`KismetSystemLibrary.K2_SetTimerDelegate` (delegate `Rotate`) 0.0 true))
  (set `self.NewVar_1` _returnvalue))

(event `Rotate`
  (bind (_returnvalue_roll _returnvalue_pitch _returnvalue_yaw) (`KismetMathLibrary.BreakRotator` (`KismetMathLibrary.RInterpTo` (`self.K2_GetActorRotation`) (`KismetMathLibrary.FindLookAtRotation` (`self.K2_GetActorLocation`) (`self.K2_GetActorLocation` (`self.Char Reference`))) (`GameplayStatics.GetWorldDeltaSeconds`) 10.0)))
  ;[1 1 1] Look at Player
  (`self.K2_SetActorRotation` (`KismetMathLibrary.MakeRotator` 0.0 0.0 _returnvalue_yaw)))

(fn `UserConstructionScript`)