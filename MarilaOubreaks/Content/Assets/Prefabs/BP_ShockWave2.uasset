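; BP_ShockWave2 is a shockwave projectile actor that damages "Enemy"-tagged actors on hit and destroys itself on any hit.
; On BeginPlay it caches the player's ThirdPersonCharacter and plays a sound at its location.
; Damage comes from the character's PlayersDamage or a fixed big-damage value when IsBigDamage is set, with a random rare roll dealing a hard-coded critical instead.
; A "Box" damage branch exists but is disconnected.
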(event `self.ReceiveBeginPlay`
  (bind _asthird_person_character (cast `/Game/Assets/ThirdPersonBP/Blueprints/ThirdPersonCharacter` (`GameplayStatics.GetPlayerCharacter` 0))
    (:`then`
      (set `self.CharRef` _asthird_person_character)
      (`GameplayStatics.PlaySoundAtLocation` null (`self.K2_GetActorLocation`) (struct) 1.0 1.0 0.0 null null null))
    (:`CastFailed`
      (`KismetSystemLibrary.PrintString` "Failed"))))

(event `self.ReceiveHit`
  (params (MyComp :type "PrimitiveComponent Object Reference") (Other :type "Actor Object Reference") (OtherComp :type "PrimitiveComponent Object Reference") (bSelfMoved :type Boolean) (HitLocation :type "Vector Structure") (HitNormal :type "Vector Structure") (NormalImpulse :type "Vector Structure") (Hit :type "HitResult Structure (by ref)"))
  (bind _charref (`self.CharRef`))
  ;[1 1 1] Main Damage Hit
  (bind _output_get (set `self.Other` Other))
  ;[1 1 1] Projectile Damage On Enemies
  (if (`self.ActorHasTag` _output_get "Enemy")
    ;[1 1 1] Set the Damages
    (if (`/Game/Assets/ThirdPersonBP/Blueprints/ThirdPersonCharacter.IsBigDamage` _charref)
      (set `self.Critical` 1000)
      (set `self.Damage` 30)
      (else
        (set `self.Critical` 1000)
        (set `self.Damage` (`KismetMathLibrary.FTrunc` (`/Game/Assets/ThirdPersonBP/Blueprints/ThirdPersonCharacter.Players_Damage` _charref)))))
    (if (== (`KismetMathLibrary.RandomIntegerInRange` 1 15) 10)
      (`GameplayStatics.ApplyDamage` _output_get 1000.0 null self "/Script/Engine.DamageType")
      (else
        (bind _returnvalue (`GameplayStatics.ApplyDamage` _output_get (`KismetMathLibrary.Conv_IntToDouble` (`self.Damage`)) null self "/Script/Engine.DamageType"))))
    (`KismetSystemLibrary.PrintString` (`KismetStringLibrary.Conv_DoubleToString` _returnvalue))
    (`self.K2_DestroyActor`)
    (else
      (`self.K2_DestroyActor`))))

(fn `UserConstructionScript`)