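; Acid hazard actor that damages and slows ThirdPersonCharacters standing inside its Radius component.
; Entering the radius starts a looping one-second ContinuousDamage timer and lowers the character's max walk speed.
; Each timer tick applies heavy damage to every overlapping ThirdPersonCharacter.
; Leaving clears the timer and sets a higher fixed walk speed, so one character exiting stops damage for any others still inside.
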(event `Continuous Damage`
  (for _array_element (`self.GetOverlappingActors` "/Game/Assets/ThirdPersonBP/Blueprints/ThirdPersonCharacter.ThirdPersonCharacter_C")
    (`GameplayStatics.ApplyDamage` _array_element 100.0 null self)))

(event `self.Radius.OnComponentBeginOverlap`
  (params (OverlappedComponent :type "PrimitiveComponent Object Reference") (OtherActor :type "Actor Object Reference") (OtherComp :type "PrimitiveComponent Object Reference") (OtherBodyIndex :type Integer) (bFromSweep :type Boolean) (SweepResult :type "HitResult Structure (by ref)"))
  (bind _asthird_person_character (cast `/Game/Assets/ThirdPersonBP/Blueprints/ThirdPersonCharacter` OtherActor))
  (`KismetSystemLibrary.K2_SetTimer` null "Continuous Damage" 1.0 true)
  (set `CharacterMovementComponent.MaxWalkSpeed` 300.0 (`Character.CharacterMovement` _asthird_person_character)))

(event `self.Radius.OnComponentEndOverlap`
  (params (OverlappedComponent :type "PrimitiveComponent Object Reference") (OtherActor :type "Actor Object Reference") (OtherComp :type "PrimitiveComponent Object Reference") (OtherBodyIndex :type Integer))
  (bind _asthird_person_character (cast `/Game/Assets/ThirdPersonBP/Blueprints/ThirdPersonCharacter` OtherActor))
  (`KismetSystemLibrary.K2_ClearTimer` null "Continuous Damage")
  (set `CharacterMovementComponent.MaxWalkSpeed` 800.0 (`Character.CharacterMovement` _asthird_person_character)))

(fn `UserConstructionScript`)