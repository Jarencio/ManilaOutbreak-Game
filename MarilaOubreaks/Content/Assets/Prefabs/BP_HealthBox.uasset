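; BP_HealthBox is a health pickup that heals the player character when it overlaps the box's sphere.
; The overlap checks for a ThirdPersonCharacter tagged Player, then a Sequence tries casts to Student, Driver and Nurse.
; Each branch adds a fixed amount of health, clamped to that class's hardcoded maximum, and prints the result.
; The box destroys itself after a matching cast, even if health is already full.
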(event `self.ReceiveBeginPlay`)

(event `self.Sphere.OnComponentBeginOverlap`
  (params (OverlappedComponent :type "PrimitiveComponent Object Reference") (OtherActor :type "Actor Object Reference") (OtherComp :type "PrimitiveComponent Object Reference") (OtherBodyIndex :type Integer) (bFromSweep :type Boolean) (SweepResult :type "HitResult Structure (by ref)"))
  (bind _asthird_person_character (cast `/Game/Assets/ThirdPersonBP/Blueprints/ThirdPersonCharacter` OtherActor))
  (if (`self.ActorHasTag` _asthird_person_character "Player")
    (`|ExecutionSequence`
      (:`then_0`
        (bind _asstudent (cast `/Game/Assets/ThirdPersonBP/Blueprints/Student` OtherActor))
        (bind _health (`/Game/Assets/ThirdPersonBP/Blueprints/ThirdPersonCharacter.Health` _asstudent))
        (if (< _health 2000.0)
          (bind _output_get (set `/Game/Assets/ThirdPersonBP/Blueprints/ThirdPersonCharacter.Health` (`KismetMathLibrary.FClamp` (+ 150.0 _health) 0.0 2000.0) _asstudent))
          (`KismetSystemLibrary.PrintString` (`KismetStringLibrary.Conv_DoubleToString` _output_get))
          (`self.K2_DestroyActor`)
          (else
            (`self.K2_DestroyActor`))))
      (:`then_1`
        (bind _asdriver (cast `/Game/Assets/ThirdPersonBP/Blueprints/Driver` OtherActor))
        (bind _health_2 (`/Game/Assets/ThirdPersonBP/Blueprints/ThirdPersonCharacter.Health` _asdriver))
        (if (< _health_2 2500.0)
          (bind _output_get_2 (set `/Game/Assets/ThirdPersonBP/Blueprints/ThirdPersonCharacter.Health` (`KismetMathLibrary.FClamp` (+ 150.0 _health_2) 0.0 2500.0) _asdriver))
          (`KismetSystemLibrary.PrintString` (`KismetStringLibrary.Conv_DoubleToString` _output_get_2))
          (`self.K2_DestroyActor`)
          (else
            (`self.K2_DestroyActor`))))
      (:`then_2`
        (bind _asnurse (cast `/Game/Assets/ThirdPersonBP/Blueprints/Nurse` OtherActor))
        (bind _health_3 (`/Game/Assets/ThirdPersonBP/Blueprints/ThirdPersonCharacter.Health` _asnurse))
        (if (< _health_3 1500.0)
          (bind _output_get_3 (set `/Game/Assets/ThirdPersonBP/Blueprints/ThirdPersonCharacter.Health` (`KismetMathLibrary.FClamp` (+ 150.0 _health_3) 0.0 1500.0) _asnurse))
          (`KismetSystemLibrary.PrintString` (`KismetStringLibrary.Conv_DoubleToString` _output_get_3))
          (`self.K2_DestroyActor`)
          (else
            (`self.K2_DestroyActor`)))))))

(fn `UserConstructionScript`)