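; Boss spawner actor that swaps the level's background music for boss music and spawns the boss enemy at its own transform.
; BossSpawn calls SpawnEnemy, which waits five seconds, then loops over every BackgroundMusic_Blueprint actor to destroy it.
; The music playback and enemy spawn sit inside that loop, so their count follows the music actors found, while NumberOfEnemy is ignored.
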(event `BossSpawn`
  (`self.Spawn Enemy` (`self.Enemy`) (`self.GetTransform`) (`self.Number of Enemy`)))

(event `self.ReceiveBeginPlay`)

(event `Spawn Enemy`
  (params (Enemy :type "Actor Class Reference") (SpawnTransform :type "Transform Structure") (`Number of Enemy` :type Integer))
  (`KismetSystemLibrary.Delay` 5.0)
  (`KismetSystemLibrary.PrintString` "Music Change")
  (bind _outactors (`GameplayStatics.GetAllActorsOfClass` "/Game/BackgroundMusic_Blueprint.BackgroundMusic_Blueprint_C"))
  (for _array_element _outactors
    (`/Game/BackgroundMusic_Blueprint.DestroySelf` _array_element)
    (`GameplayStatics.SpawnSound2D` "/Game/Music/BackgroundMusic.BackgroundMusic" 1.0 1.0 0.0 null)
    (`KismetSystemLibrary.PrintString` "Boss Music")
    (`|SpawnActorFromClass` Enemy SpawnTransform "Undefined" "OverrideRootScale" null null)))

(fn `UserConstructionScript`)