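; BP_Trash_Spawner is an actor that periodically spawns BP_Trash objects into the level.
; After an initial delay on BeginPlay, it starts a looping timer and also spawns one trash piece immediately.
; Each piece spawns at the Arrow component's world location, facing along the arrow's forward direction, at unit scale.
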(event `self.ReceiveBeginPlay`
  (`KismetSystemLibrary.Delay` (`self.Spawn First Delay`))
  (`KismetSystemLibrary.K2_SetTimerDelegate` (delegate `Spawn Trash`) (`self.Spawn Another Delay`) true)
  (`self.Spawn Trash`))

(event `Spawn Trash`
  (bind _arrow (`self.Arrow`))
  (`|SpawnActorFromClass` "/Game/Assets/Prefabs/BP_Trash.BP_Trash_C" (`KismetMathLibrary.MakeTransform` (`SceneComponent.K2_GetComponentLocation` _arrow) (`KismetMathLibrary.Conv_VectorToRotator` (`SceneComponent.GetForwardVector` _arrow))) "Undefined" "OverrideRootScale" null null))

(fn `UserConstructionScript`)