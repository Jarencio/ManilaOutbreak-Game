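; Base enemy Blueprint that roams randomly, chases seen pawns and melees the third-person character.
; PawnSensing drives AIMoveTo into a DoOnce-gated sphere-overlap attack with random montages, while a retriggerable delay resumes roaming.
; A radius overlap stores the character and sets a zero-interval looping timer for interpolated yaw facing.
; At zero health it stops movement, plays a random death montage, inflates Health, then destroys itself after a delay.
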(event `self.ReceiveBeginPlay`
  (`self.Random Roam`)
  (`GameplayStatics.PlaySoundAtLocation` null (`self.K2_GetActorLocation`) (struct) 1.0 1.0 0.0 null null null))

(event `self.ReceiveAnyDamage`
  (params (Damage :type "Float (single-precision)") (DamageType :type "DamageType Object Reference") (InstigatedBy :type "Controller Object Reference") (DamageCauser :type "Actor Object Reference"))
  (bind _death_animations (`self.Death Animations`))
  ;[1 1 1] Player damage on enemy
  (bind _output_get (set `self.Health` (`KismetMathLibrary.FClamp` (- (`self.Health`) Damage) 0.0 100.0)))
  (if (== _output_get 0.0)
    (`CharacterMovementComponent.DisableMovement` (`self.CharacterMovement`))
    (`MotionTrackedDeviceFunctionLibrary.DisableMotionTrackingOfAllControllers`)
    (`self.PlayAnimMontage` (`|GetArrayItem` _death_animations (`KismetMathLibrary.RandomInteger` (`KismetArrayLibrary.Array_Length` _death_animations))))
    (clear `self.OnActorHit`)
    (set `self.Health` 99999.0)
    (`KismetSystemLibrary.Delay` 2.5)
    (`self.K2_DestroyActor`)))

(event `Random Roam`
  ;[1 1 1] Random Roam
  (`self.PlayAnimMontage` "/Game/Animations/Enemy/Walking__3__Montage.Walking__3__Montage" 2.0)
  (`|AIMoveTo` self (`NavigationSystemV1.K2_GetRandomReachablePointInRadius` (`self.K2_GetActorLocation`) 2000.0 null null) null
    (:`OnSuccess`
      (`self.Random Roam`))))

(event `self.PawnSensing.OnSeePawn`
  (params (Pawn :type "Pawn Object Reference"))
  ;[1 1 1] Chase
  (`|ExecutionSequence`
    (:`then_0`
      (`|AIMoveTo` self (0.0 0.0 0.0) Pawn
        (:`OnSuccess`
          (`self.Attack`))))
    (:`then_1`
      (`KismetSystemLibrary.RetriggerableDelay` 1.0)
      (`self.Random Roam`))))

(event `Attack`
  (bind _attack_animations (`self.Attack Animations`))
  ;[1 1 1] Enemy attack
  (`/Engine/EditorBlueprintResources/StandardMacros.DoOnce` false :!label _label
    (:`Completed`
      (bind _outactors (`KismetSystemLibrary.SphereOverlapActors` (`SceneComponent.K2_GetComponentLocation` (`self.AttackRadius`)) 50.0 (`|MakeArray` "ObjectTypeQuery3" :!type "EObjectTypeQuery Enum") "/Game/Assets/ThirdPersonBP/Blueprints/ThirdPersonCharacter.ThirdPersonCharacter_C"))
      (for _array_element _outactors
        (`CharacterMovementComponent.DisableMovement` (`self.CharacterMovement`))
        (`|PlayMontage` (`self.Mesh`) (`|GetArrayItem` _attack_animations (`KismetMathLibrary.RandomInteger` (`KismetArrayLibrary.Array_Length` _attack_animations))) 2.0
          (:`then`
            (`GameplayStatics.ApplyDamage` _array_element (`self.Damage`) null self))
          (:`OnCompleted`
            (goto _label :!via `Reset`))
          (:`OnBlendOut`
            (`CharacterMovementComponent.SetMovementMode` (`self.CharacterMovement`) "MOVE_Walking" 0)))))))

(event `self.LookAtPlayerRadius.OnComponentBeginOverlap`
  (params (OverlappedComponent :type "PrimitiveComponent Object Reference") (OtherActor :type "Actor Object Reference") (OtherComp :type "PrimitiveComponent Object Reference") (OtherBodyIndex :type Integer) (bFromSweep :type Boolean) (SweepResult :type "HitResult Structure (by ref)"))
  ;[1 1 1] Look at Player
  (bind _ascharacter (cast `Character` OtherActor))
  (set `self.Char Reference` _ascharacter)
  (bind _returnvalue (`KismetSystemLibrary.K2_SetTimerDelegate` (delegate `Rotate`) 0.0 true))
  (set `self.NewVar_1` _returnvalue))

(event `Rotate`
  (bind (_returnvalue_roll _returnvalue_pitch _returnvalue_yaw) (`KismetMathLibrary.BreakRotator` (`KismetMathLibrary.RInterpTo` (`self.K2_GetActorRotation`) (`KismetMathLibrary.FindLookAtRotation` (`self.K2_GetActorLocation`) (`self.K2_GetActorLocation` (`self.Char Reference`))) (`GameplayStatics.GetWorldDeltaSeconds`) 10.0)))
  ;[1 1 1] Look at Player
  (`self.K2_SetActorRotation` (`KismetMathLibrary.MakeRotator` 0.0 0.0 _returnvalue_yaw)))

(fn `UserConstructionScript`)