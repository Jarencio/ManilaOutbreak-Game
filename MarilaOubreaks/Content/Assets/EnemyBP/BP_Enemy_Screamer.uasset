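; Screamer enemy that, on seeing a pawn, screams to summon a BP_EnemyBase at a random reachable point around itself.
; Sighting triggers a delayed, DoOnce-guarded scream montage and a chase move, with a retriggerable delay falling back to recursive random roaming.
; Damage spawns blood and, at zero health, plays a random death montage before destruction.
; A radius overlap sets a zero-interval timer intended to yaw it toward the character.
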(event `Random Roam`
  ;[1 1 1] Random Roam
  (`|AIMoveTo` self (`NavigationSystemV1.K2_GetRandomReachablePointInRadius` (`self.K2_GetActorLocation`) 2000.0 null null) null
    (:`OnSuccess`
      (`self.Random Roam`))))

(event `self.ReceiveAnyDamage`
  (params (Damage :type "Float (single-precision)") (DamageType :type "DamageType Object Reference") (InstigatedBy :type "Controller Object Reference") (DamageCauser :type "Actor Object Reference"))
  (bind _death_animations (`self.Death Animations`))
  ;[1 1 1] Player damage on enemy
  (`NiagaraFunctionLibrary.SpawnSystemAtLocation` "/Game/Assets/Prefabs/NS_Blood_Hit.NS_Blood_Hit" (`SceneComponent.K2_GetComponentLocation` (`self.Sphere`)))
  (bind _output_get (set `self.Health` (`KismetMathLibrary.FClamp` (- (`self.Health`) Damage) 0.0 100.0)))
  (if (== _output_get 0.0)
    (`CharacterMovementComponent.DisableMovement` (`self.CharacterMovement`))
    (`MotionTrackedDeviceFunctionLibrary.DisableMotionTrackingOfAllControllers`)
    (`self.PlayAnimMontage` (`|GetArrayItem` _death_animations (`KismetMathLibrary.RandomInteger` (`KismetArrayLibrary.Array_Length` _death_animations))))
    (clear `self.OnActorHit`)
    (set `self.Health` 99999.0)
    (`KismetSystemLibrary.Delay` 2.5)
    (`self.K2_DestroyActor`)))

(event `self.ReceiveBeginPlay`
  (`GameplayStatics.PlaySoundAtLocation` null (`self.K2_GetActorLocation`) (struct) 0.3 1.0 0.0 null null null))

(event `self.PawnSensing.OnSeePawn`
  (params (Pawn :type "Pawn Object Reference"))
  ;[1 1 1] Chase
  (`KismetSystemLibrary.Delay` 2.0)
  (`self.Attack`)
  (`|ExecutionSequence`
    (:`then_0`
      (`|AIMoveTo` self (0.0 0.0 0.0) Pawn))
    (:`then_1`
      (`KismetSystemLibrary.RetriggerableDelay` 1.0)
      (`self.Random Roam`))))

(event `Attack`
  ;[1 1 1] Enemy attack
  (`/Engine/EditorBlueprintResources/StandardMacros.DoOnce` false :!label _label
    (:`Completed`
      (`CharacterMovementComponent.DisableMovement` (`self.CharacterMovement`))
      (`|PlayMontage` (`self.Mesh`) "/Game/Animations/Enemy/Zombie_Scream__1__Montage.Zombie_Scream__1__Montage"
        (:`then`
          (`KismetSystemLibrary.Delay` 0.5)
          (`GameplayStatics.PlaySoundAtLocation` "/Game/StarterContent/Audio/Explosion01.Explosion01" (`self.K2_GetActorLocation`) (struct) 1.0 1.0 0.0 null null null)
          (`KismetSystemLibrary.Delay` 0.5)
          (`|SpawnActorFromClass` "/Game/Assets/EnemyBP/BP_EnemyBase.BP_EnemyBase_C" (`KismetMathLibrary.MakeTransform` (`NavigationSystemV1.K2_GetRandomReachablePointInRadius` (`self.K2_GetActorLocation`) 5000.0 null null)) "Undefined" "OverrideRootScale" null null))
        (:`OnCompleted`
          (goto _label :!via `Reset`))
        (:`OnBlendOut`
          (`CharacterMovementComponent.SetMovementMode` (`self.CharacterMovement`) "MOVE_Walking" 0))))))

(event `self.LookAtPlayerRadius.OnComponentBeginOverlap`
  (params (OverlappedComponent :type "PrimitiveComponent Object Reference") (OtherActor :type "Actor Object Reference") (OtherComp :type "PrimitiveComponent Object Reference") (OtherBodyIndex :type Integer) (bFromSweep :type Boolean) (SweepResult :type "HitResult Structure (by ref)"))
  ;[1 1 1] Look at Player
  (bind _ascharacter (cast `Character` OtherActor))
  (set `self.Char Reference` _ascharacter)
  (bind _returnvalue (`KismetSystemLibrary.K2_SetTimerDelegate` (delegate `Rotate`) 0.0 true))
  (set `self.NewVar_1` _returnvalue))

(event `Rotate`
  (bind (_returnvalue_roll _returnvalue_pitch _returnvalue_yaw) (`KismetMathLibrary.BreakRotator` (`KismetMathLibrary.RInterpTo` (`self.K2_GetActorRotation`) (`KismetMathLibrary.FindLookAtRotation` (`self.K2_GetActorLocation`) (`self.K2_GetActorLocation` (`self.Char Reference`))) (`GameplayStatics.GetWorldDeltaSeconds`) 10.0)))
  ;[1 1 1] Look at Player
  (`self.K2_SetActorRotation` (`KismetMathLibrary.MakeRotator` 0.0 0.0 _returnvalue_yaw)))

(fn `UserConstructionScript`)